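; Enemy light orb, a 2D flipbook hazard that travels with an InterpToMovement component and hurts Fluff characters on contact.
; It starts on the move-right flipbook and switches to move-left whenever the movement reverses, with no switch back to right.
; A growl plays at the orb's location on spawn and on each reversal.
; Overlapping its Box applies fixed damage to any Fluff_BP_Base actor.
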(event `self.ReceiveBeginPlay`
  (`PaperFlipbookComponent.SetFlipbook` (`self.Light_orb_idle`) (`self.Light_orb_move_right`))
  (`GameplayStatics.PlaySoundAtLocation` "/Game/Floors/Floors/Sound/Enemy/Light_orb_Growl.Light_orb_Growl" (`self.K2_GetActorLocation`) (struct) 1.0 1.0 0.0 null null null null :!label _label))

(event `self.InterpToMovement.OnInterpToReverse`
  (params (ImpactResult :type "HitResult Structure (by ref)") (Time :type "Float (single-precision)"))
  (`PaperFlipbookComponent.SetFlipbook` (`self.Light_orb_idle`) (`self.Light_orb_move_left`))
  (goto _label))

(event `self.Box.OnComponentBeginOverlap`
  (params (OverlappedComponent :type "PrimitiveComponent Object Reference") (OtherActor :type "Actor Object Reference") (OtherComp :type "PrimitiveComponent Object Reference") (OtherBodyIndex :type Integer) (bFromSweep :type Boolean) (SweepResult :type "HitResult Structure (by ref)"))
  (bind _asfluff_bp_base (cast `/Game/Blueprints/Light_Orbs/Fluff_BP_Base` OtherActor))
  (`GameplayStatics.ApplyDamage` _asfluff_bp_base 25.0))

(fn `UserConstructionScript`)