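; A yellow gate that opens when a PaperCharacter overlaps it while its HasKey flag is true.
; On overlap it destroys the GateClosed component, turns off collision on the trigger and both gate components, and plays the opening sound at the world origin.
; The key check and character cast each run twice in the chain, and nothing in this Blueprint sets HasKey.
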(event `self.ReceiveActorBeginOverlap`
  (params (OtherActor :type "Actor Object Reference"))
  (cast `PaperCharacter` OtherActor)
  (if (`self.HasKey`)
    (`ActorComponent.K2_DestroyComponent` (`self.Gate closed`))
    (if (`self.HasKey`)
      (cast `PaperCharacter` OtherActor)
      (`PrimitiveComponent.SetCollisionEnabled` (`self.CheckforPlayerTrigger`) "NoCollision")
      (`PrimitiveComponent.SetCollisionEnabled` (`self.Gate Open`) "NoCollision")
      (`PrimitiveComponent.SetCollisionEnabled` (`self.Gate closed`) "NoCollision")
      (`GameplayStatics.PlaySoundAtLocation` "/Game/Floors/Floors/Sound/GateOpen/Gate_Open_Sound.Gate_Open_Sound" (0.0 0.0 0.0) (struct) 1.0 1.0 0.0 null null null null))))

(fn `UserConstructionScript`)