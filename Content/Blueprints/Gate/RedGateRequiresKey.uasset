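; Red gate Blueprint that stays closed until its HasKey flag is set, then opens when a Paper2D character overlaps it.
; On actor overlap, it casts to PaperCharacter and checks HasKey, then destroys the GateClosed component, which presumably leaves GateOpen showing.
; It also disables collision on the trigger and both gate components, with a redundant second key check and cast.
; Nothing in this file sets HasKey.
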(event `self.ReceiveActorBeginOverlap`
  (params (OtherActor :type "Actor Object Reference"))
  (cast `PaperCharacter` OtherActor)
  (if (`self.HasKey`)
    (`ActorComponent.K2_DestroyComponent` (`self.Gate closed`))
    (if (`self.HasKey`)
      (cast `PaperCharacter` OtherActor)
      (`PrimitiveComponent.SetCollisionEnabled` (`self.CheckforPlayerTrigger`) "NoCollision")
      (`PrimitiveComponent.SetCollisionEnabled` (`self.Gate Open`) "NoCollision")
      (`PrimitiveComponent.SetCollisionEnabled` (`self.Gate closed`) "NoCollision"))))

(fn `UserConstructionScript`)