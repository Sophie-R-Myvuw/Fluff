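; Fluf_BP_Base is a 2D flipbook character Blueprint for side-scrolling movement along the world X axis with jumping.
; Axis input drives movement and an action drives jump and stop jumping.
; Every tick it turns the controller yaw to face the horizontal velocity direction.
; It then picks the sprite flipbook for falling, rising, walking or idle from the movement state and velocity.
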(event `self.ReceiveTick`
  (params (DeltaSeconds :type "Float (single-precision)"))
  (`|ExecutionSequence`
    (:`then_0`
      (`self.NewFunction_0`))
    (:`then_1`
      (`self.NewFunction_1`))))

(event `InputAxis|move_right`
  (params (AxisValue :type "Float (single-precision)"))
  ;[1 1 1] waking
  (`self.AddMovementInput` (1.0 0.0 0.0) AxisValue))

(event `InputAction|Jump`
  (params (Key :type "Key Structure"))
  ;[1 1 1] Comment
  (:`Pressed`
    (`self.Jump`))
  (:`Released`
    (`self.StopJumping`)))

(fn `NewFunction_0`
  (bind _returnvalue_x (`KismetMathLibrary.BreakVector` (`self.GetVelocity`)))
  (`/Engine/EditorBlueprintResources/StandardMacros.CompareFloat` _returnvalue_x
    (:`>`
      (`Controller.SetControlRotation` (`GameplayStatics.GetPlayerController` 0) (`KismetMathLibrary.MakeRotator` 0.0)))
    (:`<`
      (`Controller.SetControlRotation` (`GameplayStatics.GetPlayerController` 0) (`KismetMathLibrary.MakeRotator` 0.0 0.0 180.0)))))

(fn `NewFunction_1`
  (locals (jiump :type "PaperFlipbook Object Reference" :default "PaperFlipbook'/Game/Sprite/place_holder/flipbooks/jum_draft.jum_draft'") (walk :type "PaperFlipbook Object Reference" :default "PaperFlipbook'/Game/Sprite/place_holder/flipbooks/jump_draft.jump_draft'") (idles :type "PaperFlipbook Object Reference" :default "PaperFlipbook'/Game/Sprite/place_holder/flipbooks/idle_draft_01.idle_draft_01'"))
  (bind (_returnvalue_x _returnvalue_y _returnvalue_z) (`KismetMathLibrary.BreakVector` (`self.GetVelocity`)))
  (if (`NavMovementComponent.IsFalling` (`self.CharacterMovement`))
    (`PaperFlipbookComponent.SetFlipbook` (`self.Sprite`) (select `bool` (<= _returnvalue_z 0.0) :`false` "/Game/Sprite/place_holder/flipbooks/jum_draft.jum_draft" :`true` "/Game/Sprite/place_holder/flipbooks/fall.fall" :!type "PaperFlipbook Object Reference"))
    (elif (!= (`KismetMathLibrary.VSize` (`self.GetVelocity`)) 0.0)
      (`PaperFlipbookComponent.SetFlipbook` (`self.Sprite`) (`local.walk`))
      (else
        (`PaperFlipbookComponent.SetFlipbook` (`self.Sprite`) (`local.idles`))))))

(fn `UserConstructionScript`)