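; 2D light actor that casts a coloured, obstacle-occluded light shape and damages Fluf characters that begin overlapping its orb.
; Each tick it sweeps visibility line traces around the pitch axis, turning hit or end points into a procedural triangle fan.
; UVs encode normalised distance for the light material.
; A delayed check pushes LightColour changes to the dynamic material, and the construction script sizes the sphere to LightDistance.
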(event `self.ReceiveBeginPlay`
  ;[1 1 1] Light
  (set `self.LineTaceAngle` (/ 360.0 (`KismetMathLibrary.Conv_IntToDouble` (`self.polygon`))))
  (set `self.OriginalColour` (`self.LightColour`)))

(event `self.ReceiveTick`
  (params (DeltaSeconds :type "Float (single-precision)"))
  (bind _returnvalue (`self.K2_GetActorLocation`))
  (bind _returnvalue_2 (`self.K2_GetActorLocation`))
  (bind _vertices (`self.Vertices`))
  ;[1 1 1] Light
  (`|ExecutionSequence`
    (:`then_0`
      (`KismetArrayLibrary.Array_Clear` (`self.UV0`))
      (`KismetArrayLibrary.Array_Clear` (`self.Triangles`))
      (`KismetArrayLibrary.Array_Clear` _vertices)
      (`KismetArrayLibrary.Array_Add` _vertices)
      (`KismetArrayLibrary.Array_Add` (`self.UV0`))
      (set `self.End Vector` (`KismetMathLibrary.MakeVector` (`self.LightDistance`)))
      (for _ (range (+ (`self.polygon`) 1))
        (bind (_outhit _returnvalue_3) (`KismetSystemLibrary.LineTraceSingle` _returnvalue_2 (+ _returnvalue_2 (`self.End Vector`)) "TraceTypeQuery1"))
        (set `self.LineTraceReturn` _returnvalue_3)
        (bind (_bblockinghit _binitialoverlap _time _distance _location _impactpoint _normal _impactnormal _physmat _hitactor _hitcomponent _hitbonename _bonename _hititem _elementindex _faceindex _tracestart _traceend) (`GameplayStatics.BreakHitResult` _outhit))
        (set `self.Line Trace Location` (- _location _returnvalue))
        (set `self.Line Trace End` (- _traceend _returnvalue))
        (set `self.End Vector` (`KismetMathLibrary.GreaterGreater_VectorRotator` (`self.End Vector`) (`KismetMathLibrary.MakeRotator` 0.0 (`self.LineTaceAngle`))))
        (if (`self.LineTraceReturn`)
          (`KismetArrayLibrary.Array_Add` (`self.Vertices`) (`self.Line Trace Location`))
          (`KismetArrayLibrary.Array_Add` (`self.UV0`) (`KismetMathLibrary.MakeVector2D` (`KismetMathLibrary.MapRangeClamped` (`KismetMathLibrary.VSize` (`self.Line Trace Location`)) 0.0 (`self.LightDistance`) 0.0 1.0)))
          (else
            (`KismetArrayLibrary.Array_Add` (`self.Vertices`) (`self.Line Trace End`))
            (`KismetArrayLibrary.Array_Add` (`self.UV0`) (1.0 0.0)))))
      (set `self.TringlrOffSett` 1)
      (for _ (range (+ (- (`KismetArrayLibrary.Array_Length` (`self.Vertices`)) 3) 1))
        (`KismetArrayLibrary.Array_Add` (`self.Triangles`))
        (for _index (range 2)
          (`KismetArrayLibrary.Array_Add` (`self.Triangles`) (+ _index (`self.TringlrOffSett`))))
        (`/Engine/EditorBlueprintResources/StandardMacros.IncrementInt` (`self.TringlrOffSett`)))
      (if (`self.CreatedMesh`)
        (`ProceduralMeshComponent.UpdateMeshSection_LinearColor` :`self` (`self.ProceduralMesh`) :`Vertices` (`self.Vertices`) :`UV0` (`self.UV0`))
        (else
          (`ProceduralMeshComponent.CreateMeshSection_LinearColor` :`self` (`self.ProceduralMesh`) :`Vertices` (`self.Vertices`) :`Triangles` (`self.Triangles`) :`UV0` (`self.UV0`))
          (`PrimitiveComponent.SetMaterial` (`self.ProceduralMesh`) 0 "/Game/Blueprints/light/LightSoruce.LightSoruce")
          (bind _returnvalue_4 (`PrimitiveComponent.CreateDynamicMaterialInstance` (`self.ProceduralMesh`) 0 "/Game/Blueprints/light/LightSoruce.LightSoruce" "None"))
          (`MaterialInstanceDynamic.SetVectorParameterValue` _returnvalue_4 "LightColour" (`self.LightColour`) :!label _label))))
    (:`then_1`
      (`KismetSystemLibrary.Delay` 0.2)
      (if (not (== (`self.LightColour`) (`self.OriginalColour`)))
        (`self.UpdateColour`)
        (set `self.OriginalColour` (`self.LightColour`))))))

(event `UpdateColour`
  ;[1 1 1] Light
  (goto _label))

(event `self.Light_Orb.OnComponentBeginOverlap`
  (params (OverlappedComponent :type "PrimitiveComponent Object Reference") (OtherActor :type "Actor Object Reference") (OtherComp :type "PrimitiveComponent Object Reference") (OtherBodyIndex :type Integer) (bFromSweep :type Boolean) (SweepResult :type "HitResult Structure (by ref)"))
  ;[1 1 1] Dange
  (bind _asfluf_bp_base (cast `/Game/Blueprints/Light_Orbs/Fluf_BP_Base` OtherActor))
  (`GameplayStatics.ApplyDamage` _asfluf_bp_base 15.0))

(fn `UserConstructionScript`
  (`SphereComponent.SetSphereRadius` (`self.Light_Orb`) (`self.LightDistance`) true))